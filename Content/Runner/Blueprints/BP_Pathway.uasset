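; BP_Pathway is a path segment for an endless runner that carries a randomly chosen child actor, apparently a wall.
; On BeginPlay, SpawnWall picks one of five child-actor branches, all placed at the WallSpawnPoint transform.
; Any Box overlap asks BP_BHRGameMode to extend the ground, then slightly multiplies the player's walk speed within clamped limits and prints it.
; GetAttachPoint exposes the Arrow's world transform.
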(event OnComponentBeginOverlap(Box)
  (params (OverlappedComponent :type Primitive%20Component%20Object%20Reference) (OtherActor :type Actor%20Object%20Reference) (OtherComp :type Primitive%20Component%20Object%20Reference) (OtherBodyIndex :type Integer) (bFromSweep :type Boolean) (SweepResult :type Hit%20Result%20Structure%20%28by%20ref%29))
  ;[1 1 1] Extend The Path
  (bind _asbp_bhrgame_mode (Utilities|Casting|CastToBP_BHRGameMode (Game|GetGameMode)))
  (Default|ExtendGround _asbp_bhrgame_mode)
  ;[1 1 1] Increase Speed
  (bind _asbp_runner_player (Utilities|Casting|CastToBP_RunnerPlayer (Game|GetPlayerCharacter 0)))
  (bind _output_get (Variables|/Script/Engine.CharacterMovementComponent|SetMaxWalkSpeed (Variables|/Script/Engine.Character|GetCharacterMovement _asbp_runner_player) (Math|Float|Clamp(Float) (* (Variables|/Script/Engine.CharacterMovementComponent|GetMaxWalkSpeed (Variables|/Script/Engine.Character|GetCharacterMovement _asbp_runner_player)) 1.001) 7e+02 1.5e+03)))
  (Development|PrintString (Utilities|String|ToString(Float) _output_get)))

(event EventBeginPlay
  (CallFunction|SpawnWall))

(event Collision|EventActorBeginOverlap
  (params (OtherActor :type Actor%20Object%20Reference)))

(event EventTick
  (params (DeltaSeconds :type Float%20%28single-precision%29)))

(fn ConstructionScript)

(fn GetAttachPoint
  (return (Transformation|GetWorldTransform (Variables|Default|GetArrow))))

(fn SpawnWall
  (bind _returnvalue (CallFunction|SetSpawnPoint))
  (switch int (Math|Random|RandomIntegerinRange 0 4)
    (:0
      (AddComponent|AddChildActorComponent false _returnvalue))
    (:1
      (AddComponent|AddChildActorComponent false _returnvalue))
    (:2
      (AddComponent|AddChildActorComponent false _returnvalue))
    (:3
      (AddComponent|AddChildActorComponent false _returnvalue))
    (:4
      (AddComponent|AddChildActorComponent false _returnvalue))))

(fn SetSpawnPoint
  (return (Transformation|GetRelativeTransform (Variables|Default|GetWallSpawnPoint))))