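; BP_BHRGameMode is the runner's game mode, building and recycling the pathway the game runs on.
; On BeginPlay it spawns a starting run of BP_Pathway tiles, chaining each to the previous tile's attach point.
; ExtendGround appends a new tile and destroys the oldest once the tracked array exceeds the tile count plus one, keeping the endless track bounded.
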(event EventBeginPlay
  (for _index (range 0 (- (Variables|Default|GetNum%20of%20Tiles) 1))
    (CallFunction|AddGround)))

(event EventTick
  (params (DeltaSeconds :type Float%20%28single-precision%29)))

(fn ConstructionScript)

(fn AddGround
  (bind _returnvalue (Game|SpawnActorfromClass "/Game/Runner/Blueprints/BP_Pathway.BP_Pathway_C" (Variables|Default|GetGround%20Attach%20Point) "Undefined" "MultiplyWithRoot" 0 0))
  (bind _returnvalue_2 (Default|GetAttachPoint _returnvalue))
  (Variables|Default|SetGround%20Attach%20Point _returnvalue_2)
  (Utilities|Array|Add (Variables|Default|GetGround%20Tiles) _returnvalue))

(fn ExtendGround
  (bind _ground_tiles (Variables|Default|GetGround%20Tiles))
  (bind _output (Utilities|Array|Get(acopy) _ground_tiles))
  (CallFunction|AddGround)
  (if (> (Utilities|Array|Length (Variables|Default|GetGround%20Tiles)) (+ (Variables|Default|GetNum%20of%20Tiles) 1))
    (Actor|DestroyActor _output)
    (Utilities|Array|RemoveItem _ground_tiles _output)))